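; BP_Obstkiste is an interactable fruit box that toggles a "Use fruit box" prompt widget and responds to the item the player holds.
; An empty hand opens tutorial dialogue about Eugen's tropical fruits, unlocks an achievement through the BelvedereInstance savegame and saves.
; A filled bucket is emptied, while an empty one prompts to collect fruit first.
; Watering can, scissors and fly swatter share a "makes no sense" reply.
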(event EventBeginPlay)

(event Collision|EventActorBeginOverlap
  (params (OtherActor :type Actor%20Object%20Reference)))

(event EventTick
  (params (DeltaSeconds :type Float%20%28single-precision%29)))

(event EventInteractwith
  (params (Player :type BP%20Player%20Character%20Object%20Reference) (HeldItem :type E_Items%20Enum :default "NewEnumerator4"))
  (bind _returnvalue (Game|GetGameInstance))
  (bind _asbelvedere_instance (Utilities|Casting|CastToBelvedereInstance _returnvalue))
  (switch Utilities|FlowControl|Switch|SwitchonE_Items HeldItem
    (:NewEnumerator4
      (bind _returnvalue_2 (UserInterface|CreateWidget "/Game/UI/W_TutorialBox.W_TutorialBox_C" 0 (Utilities|Array|MakeArray "Eugen has so many tropical fruits here. 
Oranges, ananas, and lots of other citrus plants." "Some of them i have never heard of before. 
Like myrtles") 1))
      (UserInterface|Viewport|AddtoViewport _returnvalue_2 0)
      (Default|UnlockAchievement (Variables|/Game/Blueprints/BelvedereInstance.BelvedereInstance_C|GetAs%20BP%20Belvedere%20Savegame _asbelvedere_instance) "NewEnumerator3")
      (Default|SaveGame _asbelvedere_instance))
    (:NewEnumerator0
      (bind _returnvalue_3 (UserInterface|CreateWidget "/Game/UI/W_TutorialBox.W_TutorialBox_C" 0 (Utilities|Array|MakeArray "This makes no sense.") 1 :!label _label))
      (UserInterface|Viewport|AddtoViewport _returnvalue_3 0))
    (:NewEnumerator1
      (goto _label))
    (:NewEnumerator2
      (goto _label))
    (:NewEnumerator5
      (bind _full_ (Default|GetBucketFill (Variables|/Game/Blueprints/BP_PlayerCharacter.BP_PlayerCharacter_C|GetHeldItem Player)))
      (if _full_
        (Default|EmptyBucket (Variables|/Game/Blueprints/BP_PlayerCharacter.BP_PlayerCharacter_C|GetHeldItem Player))
        (else
          (bind _returnvalue_4 (UserInterface|CreateWidget "/Game/UI/W_TutorialBox.W_TutorialBox_C" 0 (Utilities|Array|MakeArray "I should collect some fruits before.") 1))
          (UserInterface|Viewport|AddtoViewport _returnvalue_4 0))))))

(event EventShowInteractMessage
  (params (TextToShow :type Text) (ShowText? :type Boolean) (HeldItem :type E_Items%20Enum :default "NewEnumerator4"))
  (bind _interactmessage (Variables|Default|GetInteractMessage))
  (Rendering|SetVisibility _interactmessage ShowText? false)
  (bind _asw_interaction_text (Utilities|Casting|CastToW_InteractionText (UserInterface|GetWidget _interactmessage)))
  (Default|SetText _asw_interaction_text "Use fruit box"))

(fn ConstructionScript)

(fn GetBucketFill
  (return false))

(fn GetFill
  (return 0.0))