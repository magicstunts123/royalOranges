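; BP_Fliegenpracker is a fly swatter tool the player picks up, described in its tutorial as a way to get rid of rotten food.
; On interaction it detaches any held item, disables its sprite physics, snaps to the player's Hand socket and registers itself as the held item.
; A DoOnce shows a tutorial box on first pickup, and the pickup chain then runs twice because both sequence outputs reach it.
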(event EventBeginPlay
  (|CallParentFunction) ; This node is disabled and will not be called.\nDrag off pins to build functionality.
)

(event Collision|EventActorBeginOverlap
  (params (OtherActor :type Actor%20Object%20Reference))
  (|CallParentFunction OtherActor) ; This node is disabled and will not be called.\nDrag off pins to build functionality.
)

(event EventTick
  (params (DeltaSeconds :type Float%20%28single-precision%29))
  (|CallParentFunction DeltaSeconds) ; This node is disabled and will not be called.\nDrag off pins to build functionality.
)

(event EventInteractwith
  (params (Player :type BP%20Player%20Character%20Object%20Reference) (HeldItem :type E_Items%20Enum :default "NewEnumerator4"))
  (bind _helditem (Variables|/Game/Blueprints/BP_PlayerCharacter.BP_PlayerCharacter_C|GetHeldItem Player)
    (:then
      (Default|DetachfromPlayer _helditem)
      (CallFunction|ShowInteractMessage "" false "NewEnumerator4"))
    (:else
      _))
  (Utilities|FlowControl|Sequence
    (:then_0
      (Utilities|FlowControl|DoOnce false
        (:Completed
          (bind _returnvalue (UserInterface|CreateWidget "/Game/UI/W_TutorialBox.W_TutorialBox_C" 0 (Utilities|Array|MakeArray "With this Fliegenpracker you  
can get rid of rotten food." "But make sure you clean afterwards.")))
          (UserInterface|Viewport|AddtoViewport _returnvalue 0))))
    (:then_1
      _))
  (|CallParentFunction Player "NewEnumerator4")
  (Physics|SetSimulatePhysics (Variables|Default|GetPaperSprite) false)
  (Transformation|AttachComponentToComponent (Variables|/Script/Paper2D.PaperCharacter|GetSprite Player) "Hand" "SnapToTarget" "SnapToTarget" "KeepWorld" false)
  (Transformation|AddLocalOffset (Variables|Default|GetPaperSprite) "0.000000,5.000000,0.000000" false false)
  (Variables|/Game/Blueprints/BP_PlayerCharacter.BP_PlayerCharacter_C|SetHeldItem Player self)
  (Variables|/Game/Blueprints/BP_PlayerCharacter.BP_PlayerCharacter_C|SetCurrentItem Player "NewEnumerator2")
  (Variables|Default|SetIsHeld true))

(fn ConstructionScript
  (|CallParentFunction))