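; BP_BaseTree is an interactable orange tree the player keeps watered and harvests, with healthy, fruiting, rotten and dead states.
; After the tutorial, looping timers lower soil moisture and raise ripeness, switching soil and tree sprites, toggling flies and killing dried-out or overripe trees.
; Interaction branches on held item: hand reports status, bucket harvests, swatter clears rot, watering can advances the tutorial once.
; AddMoisture provides clamped watering for external callers.
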(event Custom|EndTutorial
  (bind _returnvalue (Utilities|Time|SetTimerbyFunctionName 0 "Drying" 1.0 true))
  (Variables|Default|SetDryingTimerHandle _returnvalue)
  (bind _returnvalue_2 (Utilities|Time|SetTimerbyFunctionName 0 "AddReife" 1.0 true))
  (Variables|Default|SetReifeTimer _returnvalue_2)
  (Variables|Default|SetAs%20BP%20Eugen%20Mode (.AsBP%20Eugen%20Mode (Utilities|Casting|CastToBP_EugenMode (Game|GetGameMode)))))

(event EventBeginPlay)

(event Collision|EventActorBeginOverlap
  (params (OtherActor :type Actor%20Object%20Reference)))

(event EventTick
  (params (DeltaSeconds :type Float%20%28single-precision%29))
  (Rendering|Components|TextRender|SetText (Variables|Default|GetTextRender) (Utilities|Text|ToText(Float) (Variables|Default|GetFeuchte) "HalfToEven")))

(event EventShowInteractMessage
  (params (TextToShow :type Text) (ShowText? :type Boolean) (HeldItem :type E_Items%20Enum :default "NewEnumerator4"))
  (bind _interactmessage (Variables|Default|GetInteractMessage))
  (Rendering|SetVisibility _interactmessage ShowText? false)
  (bind _asw_interaction_text (Utilities|Casting|CastToW_InteractionText (UserInterface|GetWidget _interactmessage)))
  (switch Utilities|FlowControl|Switch|SwitchonE_Items HeldItem
    (:NewEnumerator4
      (Default|SetText _asw_interaction_text "Look at Tree"))
    (:NewEnumerator0
      (Default|SetText _asw_interaction_text "Pour tree"))
    (:NewEnumerator1
      (Default|SetText _asw_interaction_text "Cut tree"))
    (:NewEnumerator2
      (Default|SetText _asw_interaction_text "Hit tree!"))
    (:NewEnumerator5
      (Default|SetText _asw_interaction_text "Harvest Fruits"))))

(event EventInteractwith
  (params (Player :type BP%20Player%20Character%20Object%20Reference) (HeldItem :type E_Items%20Enum :default "NewEnumerator4"))
  (switch Utilities|FlowControl|Switch|SwitchonE_Items HeldItem
    (:NewEnumerator4
      (CallFunction|ShowStatusReport))
    (:NewEnumerator0
      (Utilities|FlowControl|DoOnce false
        (:Completed
          (Default|TutorialCounter (.AsBP%20Eugen%20Mode (Utilities|Casting|CastToBP_EugenMode (Game|GetGameMode)))))))
    (:NewEnumerator2
      (switch Utilities|FlowControl|Switch|SwitchonE_TreeState (Variables|Default|GetState)
        (:NewEnumerator0
          (bind _returnvalue (UserInterface|CreateWidget "/Game/UI/W_TutorialBox.W_TutorialBox_C" 0 (Utilities|Array|MakeArray "There is nothing i can do  
with that Fliegenpracker!") 1 :!label _label))
          (UserInterface|Viewport|AddtoViewport _returnvalue 0))
        (:NewEnumerator1
          (goto _label))
        (:NewEnumerator2
          (Variables|Default|SetReife 0.0))
        (:NewEnumerator3
          (bind _returnvalue_2 (UserInterface|CreateWidget "/Game/UI/W_TutorialBox.W_TutorialBox_C" 0 (Utilities|Array|MakeArray "There is no hope for this one. 
I hope Eugen will not be that angry about it.") 1 :!label _label_2))
          (UserInterface|Viewport|AddtoViewport _returnvalue_2 0))))
    (:NewEnumerator5
      (switch Utilities|FlowControl|Switch|SwitchonE_TreeState (Variables|Default|GetState)
        (:NewEnumerator0
          (bind _returnvalue_3 (UserInterface|CreateWidget "/Game/UI/W_TutorialBox.W_TutorialBox_C" 0 (Utilities|Array|MakeArray "Here are no fruits to collect! 
I have to wait a bit. 
") 1))
          (UserInterface|Viewport|AddtoViewport _returnvalue_3 0))
        (:NewEnumerator1
          (bind _full_ (Default|GetBucketFill (Variables|/Game/Blueprints/BP_PlayerCharacter.BP_PlayerCharacter_C|GetHeldItem Player)))
          (if _full_
            (bind _returnvalue_4 (UserInterface|CreateWidget "/Game/UI/W_TutorialBox.W_TutorialBox_C" 0 (Utilities|Array|MakeArray "The Bucket is already full! 
I need to emty it first!") 1))
            (UserInterface|Viewport|AddtoViewport _returnvalue_4 0)
            (else
              (Variables|Default|SetReife 0.0)
              (Default|FillBucket (Variables|/Game/Blueprints/BP_PlayerCharacter.BP_PlayerCharacter_C|GetHeldItem Player))
              (Niagara|SpawnSystematLocation "/Game/Blueprints/NS_Oranges.NS_Oranges" (Transformation|GetWorldLocation (Variables|Default|GetScene))))))
        (:NewEnumerator2
          (bind _returnvalue_5 (UserInterface|CreateWidget "/Game/UI/W_TutorialBox.W_TutorialBox_C" 0 (Utilities|Array|MakeArray "Am I crazy? 
I cannot collect rotten  
food for our guests!") 1))
          (UserInterface|Viewport|AddtoViewport _returnvalue_5 0))
        (:NewEnumerator3
          (goto _label_2))))))

(fn ConstructionScript)

(fn SetStateOfTree
  (params (State :type E_TreeState%20Enum :default "NewEnumerator0"))
  (bind _as_bp_eugen_mode (Variables|Default|GetAs%20BP%20Eugen%20Mode))
  (bind _output_get (Variables|Default|SetState State))
  (switch Utilities|FlowControl|Switch|SwitchonE_TreeState _output_get
    (:NewEnumerator0
      (CallFunction|ShowSprites true false false))
    (:NewEnumerator1
      (Utilities|FlowControl|Sequence
        (:then_0
          (Default|ShowBucketTutorial _as_bp_eugen_mode))
        (:then_1
          _))
      (CallFunction|ShowSprites false true false))
    (:NewEnumerator2
      (Utilities|FlowControl|Sequence
        (:then_0
          (Default|ShowPrackerTutorial _as_bp_eugen_mode))
        (:then_1
          _))
      (CallFunction|ShowSprites false false true))
    (:NewEnumerator3
      (Rendering|Components|Sprite|SetSprite (Variables|Default|GetBaum) "/Game/Assets/tot_Sprite.tot_Sprite")
      (CallFunction|ShowSprites true false false)
      (Utilities|Time|ClearandInvalidateTimerbyHandle (Variables|Default|GetReifeTimer)))))

(fn ShowSprites
  (params (bShowTree :type Boolean) (bShowOranges :type Boolean) (bShowKaputteOranges :type Boolean))
  (Rendering|SetVisibility (Variables|Default|GetBaum) bShowTree false)
  (Rendering|SetVisibility (Variables|Default|GetOrangen) bShowOranges false)
  (Rendering|SetVisibility (Variables|Default|GetVerdorbenSprite) bShowKaputteOranges false))

(fn Drying
  (bind _output_get (Variables|Default|SetFeuchte (- (Variables|Default|GetFeuchte) (Math|Random|RandomFloatinRange 1.0 2.0))))
  (if (<= _output_get 0.0)
    (CallFunction|SetStateOfTree "NewEnumerator3")
    (Development|PrintString "dead")
    (Rendering|Components|Sprite|SetSprite (Variables|Default|GetErde) "/Game/Assets/Erde_0_Sprite.Erde_0_Sprite")
    (elif (Math|Float|InRange(Float) (Variables|Default|GetFeuchte) 8e+01 1e+02)
      (Rendering|Components|Sprite|SetSprite (Variables|Default|GetErde) "/Game/Assets/Erde_100_Sprite.Erde_100_Sprite")
      (elif (Math|Float|InRange(Float) (Variables|Default|GetFeuchte) 5e+01 8e+01)
        (Rendering|Components|Sprite|SetSprite (Variables|Default|GetErde) "/Game/Assets/Erde_50_Sprite.Erde_50_Sprite")
        (elif (Math|Float|InRange(Float) (Variables|Default|GetFeuchte) 5e+01 1e+02)
          (Rendering|Components|Sprite|SetSprite (Variables|Default|GetErde) "/Game/Assets/Erde_20_Sprite.Erde_20_Sprite"))))))

(fn AddReife
  (bind _flies (Variables|Default|GetFlies))
  (bind _output_get (Variables|Default|SetReife (+ (Variables|Default|GetReife) (Math|Random|RandomFloatinRange 1.0 3.0))))
  (if (> _output_get 8e+01)
    (if (> (Variables|Default|GetReife) 1.1e+02)
      (if (> (Variables|Default|GetReife) 1.1e+02)
        (if (> (Variables|Default|GetReife) 1.3e+02)
          (CallFunction|SetStateOfTree "NewEnumerator3")
          (else
            (CallFunction|SetStateOfTree "NewEnumerator2")
            (Components|Activation|Activate _flies false)))
        (else
          (CallFunction|SetStateOfTree "NewEnumerator1")
          (Components|Activation|Deactivate _flies :!label _label)))
      (else
        (CallFunction|SetStateOfTree "NewEnumerator1")
        (goto _label)))
    (else
      (CallFunction|SetStateOfTree "NewEnumerator0")
      (Components|Activation|Deactivate _flies))))

(fn ShowStatusReport
  (bind _feuchte (Variables|Default|GetFeuchte))
  (switch Utilities|FlowControl|Switch|SwitchonE_TreeState (Variables|Default|GetState)
    (:NewEnumerator0
      (LocalVariables|SetStateDescription "The tree is in good shape.")
      (LocalVariables|SetStateDescription2 "Otherwise the tree is in good shape."))
    (:NewEnumerator1
      (LocalVariables|SetStateDescription "The tree has fruits! Get them!")
      (LocalVariables|SetStateDescription2 "The tree has fruits! Get them!"))
    (:NewEnumerator2
      (LocalVariables|SetStateDescription "The fruits are already in a bad shape. 
Better get rid of them!")
      (LocalVariables|SetStateDescription2 "The fruits are already in a bad shape. 
Better get rid of them!"))
    (:NewEnumerator3
      (LocalVariables|SetStateDescription "This tree is dead. Eugen will not be happy about this!")
      (LocalVariables|SetStateDescription2 "This tree is dead. Eugen will not be happy about this!")))
  (if (> _feuchte 6e+01)
    (bind _returnvalue (UserInterface|CreateWidget "/Game/UI/W_TutorialBox.W_TutorialBox_C" 0 (Utilities|Array|MakeArray (Utilities|Text|FormatText "This soil is wet. ({Value}%) 
{Description}" _feuchte (LocalVariables|GetStateDescription))) 1))
    (UserInterface|Viewport|AddtoViewport _returnvalue 0)
    (else
      (bind _returnvalue_2 (UserInterface|CreateWidget "/Game/UI/W_TutorialBox.W_TutorialBox_C" 0 (Utilities|Array|MakeArray (Utilities|Text|FormatText "This soil is getting dry! ({Value}%) 
You should get some water! 
{Description}" _feuchte (LocalVariables|GetStateDescription2))) 1))
      (UserInterface|Viewport|AddtoViewport _returnvalue_2 0))))

(fn AddMoisture
  (params (Value :type Float%20%28double-precision%29))
  (Variables|Default|SetFeuchte (Math|Float|Clamp(Float) (+ (Variables|Default|GetFeuchte) Value) 0.0 1e+02)))

(fn GetBucketFill
  (return false))

(fn GetFill
  (return 0.0))