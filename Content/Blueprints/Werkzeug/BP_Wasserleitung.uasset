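; BP_Wasserleitung is an interactable water pipe that shows a "Use water" prompt and reacts to the held item.
; Interacting by hand shows dialogue about the Hofburg's water source and unlocks an achievement through BelvedereInstance.
; Scissors, fly swatter and bucket each get a refusal line in a W_TutorialBox.
; The filling event is empty and the fill getters return false and zero, so it never fills anything.
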(event Custom|Filling)

(event EventBeginPlay)

(event Collision|EventActorBeginOverlap
  (params (OtherActor :type Actor%20Object%20Reference)))

(event EventTick
  (params (DeltaSeconds :type Float%20%28single-precision%29)))

(event EventInteractwith
  (params (Player :type BP%20Player%20Character%20Object%20Reference) (HeldItem :type E_Items%20Enum :default "NewEnumerator4"))
  (switch Utilities|FlowControl|Switch|SwitchonE_Items HeldItem
    (:NewEnumerator4
      (bind _returnvalue (UserInterface|CreateWidget "/Game/UI/W_TutorialBox.W_TutorialBox_C" 0 (Utilities|Array|MakeArray "Money can make nearly anything possible." "I heard this water is from the Siebenbrunner Hofwasserleitung. 
This is the same water they use in the Hofburg!") 1))
      (UserInterface|Viewport|AddtoViewport _returnvalue 0)
      (Default|UnlockAchievement (.AsBelvedere%20Instance (Utilities|Casting|CastToBelvedereInstance (Game|GetGameInstance))) "NewEnumerator4"))
    (:NewEnumerator1
      (bind _returnvalue_2 (UserInterface|CreateWidget "/Game/UI/W_TutorialBox.W_TutorialBox_C" 0 (Utilities|Array|MakeArray "This makes no sense.") 1 :!label _label))
      (UserInterface|Viewport|AddtoViewport _returnvalue_2 0))
    (:NewEnumerator2
      (goto _label))
    (:NewEnumerator5
      (bind _returnvalue_3 (UserInterface|CreateWidget "/Game/UI/W_TutorialBox.W_TutorialBox_C" 0 (Utilities|Array|MakeArray "I should use something else to water the trees.") 1))
      (UserInterface|Viewport|AddtoViewport _returnvalue_3 0))))

(event EventShowInteractMessage
  (params (TextToShow :type Text) (ShowText? :type Boolean) (HeldItem :type E_Items%20Enum :default "NewEnumerator4"))
  (bind _interactmessage (Variables|Default|GetInteractMessage))
  (Rendering|SetVisibility _interactmessage ShowText? false)
  (bind _asw_interaction_text (Utilities|Casting|CastToW_InteractionText (UserInterface|GetWidget _interactmessage)))
  (Default|SetText _asw_interaction_text "Use water"))

(fn ConstructionScript)

(fn GetBucketFill
  (return false))

(fn GetFill
  (return 0.0))