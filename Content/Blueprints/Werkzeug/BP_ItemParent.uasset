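; Base Blueprint for holdable Paper2D items that return to their starting spot after being dropped.
; It records its transform at BeginPlay; detaching enables sprite physics, then a retriggerable 10-second delay calls ResetItem, which restores that transform unless the item is held.
; A widget component shows or hides the item's own interaction text.
; GetBucketFill and GetFill return empty defaults, apparently for child items to override.
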(event Custom|DetachFromPlayer
  (Transformation|AddLocalOffset (Variables|Default|GetPaperSprite) "0.000000,-5.000000,0.000000" false false)
  (Transformation|DetachFromActor "KeepWorld" "KeepWorld" "KeepWorld")
  (Physics|SetSimulatePhysics (Variables|Default|GetPaperSprite) true)
  (Variables|Default|SetIsHeld false)
  (Utilities|FlowControl|RetriggerableDelay 1e+01)
  (CallFunction|ResetItem))

(event Custom|ResetItem
  (if (not (Variables|Default|GetIsHeld))
    (Transformation|SetActorTransform (Variables|Default|GetInitTransform))
    (Physics|SetSimulatePhysics (Variables|Default|GetPaperSprite) false)))

(event EventBeginPlay
  (Variables|Default|SetInitTransform (Transformation|GetActorTransform)))

(event Collision|EventActorBeginOverlap
  (params (OtherActor :type Actor%20Object%20Reference)))

(event EventTick
  (params (DeltaSeconds :type Float%20%28single-precision%29)))

(event EventShowInteractMessage
  (params (TextToShow :type Text) (ShowText? :type Boolean) (HeldItem :type E_Items%20Enum :default "NewEnumerator4"))
  (bind _interactmessage (Variables|Default|GetInteractMessage))
  (Rendering|SetVisibility _interactmessage ShowText? false)
  (bind _asw_interaction_text (Utilities|Casting|CastToW_InteractionText (UserInterface|GetWidget _interactmessage)))
  (Default|SetText _asw_interaction_text (Variables|Default|GetOwnInteractionText)))

(fn ConstructionScript)

(fn GetBucketFill
  (return false))

(fn GetFill
  (return 0.0))