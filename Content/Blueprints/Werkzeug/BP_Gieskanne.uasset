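; Watering can item that the player picks up and refills, tracking a clamped water level exposed through GetFill.
; Interacting drops any held item, attaches the can to the player's Hand socket and shows the HUD watering bar, with a tutorial box on first pickup; detaching hides the bar.
; FillUpCan updates the bar and plays a hose sound once, using a retriggerable delay to fade it out when filling stops.
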(event Collision|EventActorBeginOverlap
  (params (OtherActor :type Actor%20Object%20Reference))
  (|CallParentFunction OtherActor) ; This node is disabled and will not be called.\nDrag off pins to build functionality.
)

(event EventInteractwith
  (params (Player :type BP%20Player%20Character%20Object%20Reference) (HeldItem :type E_Items%20Enum :default "NewEnumerator4"))
  (bind _helditem (Variables|/Game/Blueprints/BP_PlayerCharacter.BP_PlayerCharacter_C|GetHeldItem Player)
    (:then
      (Default|DetachfromPlayer _helditem)
      (CallFunction|ShowInteractMessage "" false "NewEnumerator4"))
    (:else
      _))
  (Utilities|FlowControl|Sequence
    (:then_0
      (Utilities|FlowControl|DoOnce false
        (:Completed
          (bind _returnvalue (UserInterface|CreateWidget "/Game/UI/W_TutorialBox.W_TutorialBox_C" 0 (Utilities|Array|MakeArray "Great! You are really good following orders! 
Now water the trees one by one!")))
          (UserInterface|Viewport|AddtoViewport _returnvalue 0))))
    (:then_1
      _))
  (|CallParentFunction Player "NewEnumerator4")
  (Physics|SetSimulatePhysics (Variables|Default|GetPaperSprite) false)
  (Transformation|AttachComponentToComponent (Variables|/Script/Paper2D.PaperCharacter|GetSprite Player) "Hand" "SnapToTarget" "SnapToTarget" "KeepWorld" false)
  (Transformation|AddLocalOffset (Variables|Default|GetPaperSprite) "0.000000,5.000000,0.000000" false false)
  (Variables|/Game/Blueprints/BP_PlayerCharacter.BP_PlayerCharacter_C|SetHeldItem Player self)
  (Variables|/Game/Blueprints/BP_PlayerCharacter.BP_PlayerCharacter_C|SetCurrentItem Player "NewEnumerator0")
  (Variables|Default|SetIsHeld true)
  (Default|ShowWateringBar (Variables|/Game/Blueprints/BP_EugenMode.BP_EugenMode_C|GetHUD (Variables|Default|GetAs%20BP%20Eugen%20Mode)) "Visible"))

(event EventFillUpCan
  (params (Value :type Float%20%28double-precision%29))
  (bind _output_get (Variables|Default|SetWater (Math|Float|Clamp(Float) (+ (Variables|Default|GetWater) Value) 0.0 1e+02)))
  (Default|UpdateWateringBar (Variables|/Game/Blueprints/BP_EugenMode.BP_EugenMode_C|GetHUD (Variables|Default|GetAs%20BP%20Eugen%20Mode)) _output_get)
  (Utilities|FlowControl|Sequence
    (:then_0
      (Utilities|FlowControl|DoOnce false :!label _label
        (:Completed
          (bind _returnvalue (Audio|SpawnSound2D "/Game/Assets/Audio/Wasserschlauch_Cue.Wasserschlauch_Cue" 1.0 1.0 0.0 0))
          (Variables|Default|SetWassSound _returnvalue))))
    (:then_1
      (Utilities|FlowControl|RetriggerableDelay 0.2)
      (bind _wasssound (Variables|Default|GetWassSound)
        (:then
          (Audio|Components|Audio|FadeOut _wasssound 0.2 0.0 "Linear" :!class /Script/Engine.AudioComponent)
          (goto _label Reset))
        (:else
          (goto _label Reset))))))

(event EventBeginPlay
  (|CallParentFunction)
  (bind _asbp_eugen_mode (Utilities|Casting|CastToBP_EugenMode (Game|GetGameMode)))
  (Variables|Default|SetAs%20BP%20Eugen%20Mode _asbp_eugen_mode))

(event EventDetachfromPlayer
  (|CallParentFunction)
  (Default|ShowWateringBar (Variables|/Game/Blueprints/BP_EugenMode.BP_EugenMode_C|GetHUD (Variables|Default|GetAs%20BP%20Eugen%20Mode)) "Hidden"))

(fn ConstructionScript
  (|CallParentFunction))

(fn GetFill
  (return (Variables|Default|GetWater)))