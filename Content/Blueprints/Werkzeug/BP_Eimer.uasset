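; BP_Eimer is a bucket tool the player carries, described by its tutorial as the means of harvesting fruit.
; Interacting detaches any held item, shows a one-time tutorial widget, then attaches the physics-disabled sprite to the player's Hand socket and registers it as the held item.
; FillBucket and EmptyBucket toggle the Full flag and swap the Paper2D sprite, with GetBucketFill exposing that state.
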(event EventBeginPlay
  (|CallParentFunction) ; This node is disabled and will not be called.\nDrag off pins to build functionality.
)

(event Collision|EventActorBeginOverlap
  (params (OtherActor :type Actor%20Object%20Reference))
  (|CallParentFunction OtherActor) ; This node is disabled and will not be called.\nDrag off pins to build functionality.
)

(event EventTick
  (params (DeltaSeconds :type Float%20%28single-precision%29))
  (|CallParentFunction DeltaSeconds) ; This node is disabled and will not be called.\nDrag off pins to build functionality.
)

(event EventInteractwith
  (params (Player :type BP%20Player%20Character%20Object%20Reference) (HeldItem :type E_Items%20Enum :default "NewEnumerator4"))
  (bind _helditem (Variables|/Game/Blueprints/BP_PlayerCharacter.BP_PlayerCharacter_C|GetHeldItem Player)
    (:then
      (Default|DetachfromPlayer _helditem))
    (:else
      _))
  (CallFunction|ShowInteractMessage "" false "NewEnumerator4")
  (Utilities|FlowControl|Sequence
    (:then_0
      (Utilities|FlowControl|DoOnce false
        (:Completed
          (bind _returnvalue (UserInterface|CreateWidget "/Game/UI/W_TutorialBox.W_TutorialBox_C" 0 (Utilities|Array|MakeArray "With this Bucket you can harvest fruits!" "You shall do this before the fruits are too old!")))
          (UserInterface|Viewport|AddtoViewport _returnvalue 0))))
    (:then_1
      _))
  (|CallParentFunction Player "NewEnumerator4")
  (Physics|SetSimulatePhysics (Variables|Default|GetPaperSprite) false)
  (Transformation|AttachComponentToComponent (Variables|/Script/Paper2D.PaperCharacter|GetSprite Player) "Hand" "SnapToTarget" "SnapToTarget" "KeepWorld" false)
  (Transformation|AddLocalOffset (Variables|Default|GetPaperSprite) "0.000000,5.000000,0.000000" false false)
  (Variables|/Game/Blueprints/BP_PlayerCharacter.BP_PlayerCharacter_C|SetHeldItem Player self)
  (Variables|/Game/Blueprints/BP_PlayerCharacter.BP_PlayerCharacter_C|SetCurrentItem Player "NewEnumerator5")
  (Variables|Default|SetIsHeld true))

(event EventFillUpCan
  (params (Value :type Float%20%28double-precision%29)))

(event EventFillBucket
  (Variables|Default|SetbFull? true)
  (Rendering|Components|Sprite|SetSprite (Variables|Default|GetPaperSprite) "/Game/Assets/Kubel_gefullt_Sprite.Kubel_gefullt_Sprite"))

(event EventEmptyBucket
  (Variables|Default|SetbFull? false)
  (Rendering|Components|Sprite|SetSprite (Variables|Default|GetPaperSprite) "/Game/Assets/Kubel_Sprite.Kubel_Sprite"))

(fn ConstructionScript
  (|CallParentFunction))

(fn GetBucketFill
  (return (Variables|Default|GetbFull?)))