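; BP_BelvedereSavegame is the save-game Blueprint for the Belvedere game, recording which achievements are unlocked.
; Its UnlockAchievement event switches on the achievement, whose cases include titled works such as Siege Of Belgrade (1717) and entries such as Eugenia.
; Each case sets a save-struct member to true at its own fixed index in the Unlockables array.
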(event Custom|UnlockAchievement
  (params (Achievement :type E_Achievement%20Enum :default "NewEnumerator0"))
  (switch Utilities|FlowControl|Switch|SwitchonE_Achievement Achievement
    (:NewEnumerator0
      (Utilities|Struct|SetmembersinS_Savestruct (Utilities|Array|Get(acopy) (Variables|Default|GetUnlockables)) true))
    (:NewEnumerator1
      (Utilities|Struct|SetmembersinS_Savestruct (Utilities|Array|Get(acopy) (Variables|Default|GetUnlockables) 1) true))
    (:NewEnumerator2
      (Utilities|Struct|SetmembersinS_Savestruct (Utilities|Array|Get(acopy) (Variables|Default|GetUnlockables) 2) true))
    (:NewEnumerator3
      (Utilities|Struct|SetmembersinS_Savestruct (Utilities|Array|Get(acopy) (Variables|Default|GetUnlockables) 3) true))
    (:NewEnumerator4
      (Utilities|Struct|SetmembersinS_Savestruct (Utilities|Array|Get(acopy) (Variables|Default|GetUnlockables) 4) true))))