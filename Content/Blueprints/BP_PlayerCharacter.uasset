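; Player character for a 2D gardener: moves along one axis with a mirrored flipbook sprite, idle/walk animation and throttled step sounds.
; A per-Tick sphere trace along the negative right vector finds BPI_Interaction actors, using paired DoOnce gates to toggle their prompts.
; Interact messages the target with the current item; holding it with the watering can refills at water pipes or moistens trees.
; Left click drops the held item, and Escape opens the pause widget.
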(event Input|EnhancedActionEvents|EnhancedInputActionIA_Move
  (params (ActionValue :type Vector%202D%20Structure) (ElapsedSeconds :type Float%20%28double-precision%29) (TriggeredSeconds :type Float%20%28double-precision%29) (InputAction :type Input%20Action%20Object%20Reference :default "/Game/Blueprints/Input/IA_Move.IA_Move"))
  ;[1 1 1] Movement
  (CallFunction|SetSpriteDirection (.x ActionValue))
  (Pawn|Input|AddMovementInput (Math|Vector|MakeVector (.x ActionValue) 0.0 0.0) 1.0 false)
  (Utilities|FlowControl|DoOnce false :!label _label
    (:Completed
      (bind _returnvalue (Audio|SpawnSound2D "/Game/Assets/Audio/TokV1.TokV1" 2.0 1.0 0.0 0))
      (Variables|Default|SetTockSound _returnvalue)
      (Utilities|FlowControl|Delay 0.3)
      (goto _label Reset))))

(event Input|EnhancedActionEvents|EnhancedInputActionIA_Interact
  (params (ActionValue :type Boolean) (ElapsedSeconds :type Float%20%28double-precision%29) (TriggeredSeconds :type Float%20%28double-precision%29) (InputAction :type Input%20Action%20Object%20Reference :default "/Game/Blueprints/Input/IA_Interact.IA_Interact"))
  (bind _returnvalue (Utilities|Time|GetWorldDeltaSeconds))
  (bind _helditem (Variables|Default|GetHeldItem))
  (bind _returnvalue_2 (* _returnvalue -2e+01))
  (:Triggered
    (switch Utilities|FlowControl|Switch|SwitchonE_Items (Variables|Default|GetCurrentItem)
      (:NewEnumerator0
        (Utilities|Casting|CastToBP_Wasserleitung (Variables|Default|GetLookAtActor)
          (:then
            (Default|FillUpCan (Variables|Default|GetHeldItem) (* (Utilities|Time|GetWorldDeltaSeconds) 15.0)))
          (:CastFailed
            (bind _asbp_base_tree (Utilities|Casting|CastToBP_BaseTree (Variables|Default|GetLookAtActor)))
            (bind _value (Default|GetFill _helditem))
            (if (> _value 0.0)
              (Default|FillUpCan _helditem _returnvalue_2)
              (Default|AddMoisture _asbp_base_tree (* _returnvalue_2 -1.0))))))))
  (:Started
    (bind _lookatactor (Variables|Default|GetLookAtActor)
      (:then
        (Class|BPIInteraction|Interactwith(Message) _lookatactor self (Variables|Default|GetCurrentItem)))
      (:else))))

(event Collision|EventActorBeginOverlap
  (params (OtherActor :type Actor%20Object%20Reference)))

(event EventBeginPlay
  (bind _asbp_eugen_mode (Utilities|Casting|CastToBP_EugenMode (Game|GetGameMode)))
  (Variables|Default|SetAs%20BP%20Eugen%20Mode _asbp_eugen_mode))

(event EventTick
  (params (DeltaSeconds :type Float%20%28single-precision%29))
  (bind _returnvalue (Transformation|GetActorLocation))
  (bind _currentitem (Variables|Default|GetCurrentItem))
  (CallFunction|HandleAnimation)
  (bind (_outhit _returnvalue_2) (Collision|SphereTraceByChannel _returnvalue (+ _returnvalue (* (* (Transformation|GetActorRightVector) "-1.000000,-1.000000,-1.000000") 5e+03)) 5e+01 "TraceTypeQuery1" false (Utilities|Array|MakeArray (Variables|Default|GetHeldItem)) "None"))
  (if _returnvalue_2
    (if (Utilities|DoesObjectImplementInterface (.HitActor (Collision|BreakHitResult _outhit)) "/Game/Blueprints/BPI_Interaction.BPI_Interaction_C")
      (Variables|Default|SetLookAtActor (.HitActor (Collision|BreakHitResult _outhit)))
      (Utilities|FlowControl|DoOnce false :!label _label
        (:Completed
          (Class|BPIInteraction|ShowInteractMessage(Message) (Variables|Default|GetLookAtActor) "Interact" true _currentitem)
          (goto _label_2 Reset)))
      (else
        _)))
  (Utilities|FlowControl|DoOnce false :!label _label_2
    (:Completed
      (bind _lookatactor (Variables|Default|GetLookAtActor)
        (:then
          (Class|BPIInteraction|ShowInteractMessage(Message) _lookatactor "Interact" false _currentitem)
          (goto _label Reset))
        (:else)))))

(event Input|MouseEvents|LeftMouseButton
  (params (Key :type Key%20Structure :default "None"))
  (:Pressed
    (bind _helditem (Variables|Default|GetHeldItem)
      (:then
        (Default|DetachfromPlayer _helditem)
        (Variables|Default|SetHeldItem 0)
        (Variables|Default|SetCurrentItem "NewEnumerator4"))
      (:else))))

(event Input|KeyboardEvents|Escape
  (params (Key :type Key%20Structure :default "None"))
  (:Pressed
    (bind _returnvalue (UserInterface|CreateWidget "/Game/UI/W_Pause.W_Pause_C"))
    (UserInterface|Viewport|AddtoViewport _returnvalue 0)))

(fn ConstructionScript)

(fn SetIdleAnim
  (params (ShouldIdle :type Boolean))
  (bind _sprite (Variables|Default|GetSprite))
  (if ShouldIdle
    (Utilities|FlowControl|DoOnce false :!label _label
      (:Completed
        (Sprite|SetFlipbook _sprite "/Game/Assets/gaertner_stehend_Flipbook.gaertner_stehend_Flipbook") ; Hier kommt Idle rein
        (goto _label_2 Reset)))
    (else
      (Utilities|FlowControl|DoOnce false :!label _label_2
        (:Completed
          (Sprite|SetFlipbook _sprite "/Game/Assets/gartner_walk.gartner_walk") ; Hier kommt Run
          (goto _label Reset))))))

(fn SetSpriteDirection
  (params (XMovement :type Float%20%28double-precision%29))
  (bind _sprite (Variables|Default|GetSprite))
  (if (< XMovement 0.0)
    (Transformation|SetRelativeScale3D _sprite "-0.150000,0.150000,0.150000")
    (else
      (Transformation|SetRelativeScale3D _sprite "0.150000,0.150000,0.150000"))))

(fn HandleAnimation
  (CallFunction|SetIdleAnim (== (Math|Vector|VectorLength (Transformation|GetVelocity)) 0.0)))