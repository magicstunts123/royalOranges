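; Game mode for an orangerie gardening game that runs the tutorial and the visits of the NPC Eugen.
; BeginPlay caches all trees and Eugen, starts music, shows the HUD and opens intro dialogue.
; A watering counter ends the tutorial and sends Eugen away on a timer, resuming tree timers.
; His return pauses those timers and switches to stress music; one-shot events show bucket and fly-swatter hints.
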(event Custom|ShowBucketTutorial
  (Utilities|FlowControl|DoOnce false
    (:Completed
      (bind _returnvalue (UserInterface|CreateWidget "/Game/UI/W_TutorialBox.W_TutorialBox_C" 0 (Utilities|Array|MakeArray "A tree got some fruits! 
I should collect them with the bucket!" "...before the fruits rot!") 1))
      (UserInterface|Viewport|AddtoViewport _returnvalue 0))))

(event Custom|EugenMoveAway
  (Default|GoAway (Variables|Default|GetEugenNPC))
  (CallFunction|StartEugenAwayTimer)
  (CallFunction|StartTreeTimers)
  (bind _stressmuic (Variables|Default|GetStressMuic)
    (:then
      (Audio|Components|Audio|FadeOut _stressmuic 2.0 0.0 "Linear" :!class /Script/Engine.AudioComponent))
    (:else
      _))
  (Utilities|FlowControl|Delay 1.0)
  (if (not (Audio|Components|Audio|IsPlaying (Variables|Default|GetBGMMusic)))
    (bind _returnvalue (Audio|SpawnSound2D "/Game/Assets/Audio/BGM.BGM" 1.0 1.0 0.0 0 false false))
    (Variables|Default|SetBGMMusic _returnvalue)))

(event Custom|EugenComeBack
  (Default|ComeBack (Variables|Default|GetEugenNPC))
  (CallFunction|StopTreeTimers)
  (Audio|Components|Audio|FadeOut (Variables|Default|GetBGMMusic) 2.0 0.0 "Linear" :!class /Script/Engine.AudioComponent)
  (Utilities|FlowControl|Delay 1.0)
  (bind _returnvalue (Audio|SpawnSound2D "/Game/Assets/Audio/nelly-julio-salvador-sagreras-1879-1942-arranged-for-strings-189991_Cue.nelly-julio-salvador-sagreras-1879-1942-arranged-for-strings-189991_Cue" 1.0 1.0 0.0 0))
  (Variables|Default|SetStressMuic _returnvalue))

(event Custom|StartEugenAwayTimer
  (bind _returnvalue (Utilities|Time|SetTimerbyEvent (delegate Custom|EugenComeBack) 3e+01))
  (Variables|Default|SetTimer _returnvalue))

(event Custom|ShowPrackerTutorial
  (Utilities|FlowControl|DoOnce false
    (:Completed
      (bind _returnvalue (UserInterface|CreateWidget "/Game/UI/W_TutorialBox.W_TutorialBox_C" 0 (Utilities|Array|MakeArray "Oh no! The Fruits of one tree got rotten! 
Is should remove them with the Fliegenpracker!") 1))
      (UserInterface|Viewport|AddtoViewport _returnvalue 0))))

(event EventBeginPlay
  (bind _outactors (Actor|GetAllActorsOfClass "/Game/Blueprints/Werkzeug/BP_BaseTree.BP_BaseTree_C"))
  (Variables|Default|SetTrees _outactors)
  (bind _returnvalue (Audio|SpawnSound2D "/Game/Assets/Audio/BGM.BGM" 1.0 1.0 0.0 0 false false))
  (Variables|Default|SetBGMMusic _returnvalue)
  (bind _returnvalue_2 (UserInterface|CreateWidget "/Game/UI/W_GameHUD.W_GameHUD_C"))
  (UserInterface|Viewport|AddtoViewport _returnvalue_2 0)
  (Variables|Default|SetHUD _returnvalue_2)
  (Utilities|FlowControl|Delay 0.2)
  (bind _returnvalue_3 (UserInterface|CreateWidget "/Game/UI/W_TutorialBox.W_TutorialBox_C" 0 (Utilities|Array|MakeArray "Hello! I am Eugen! 
You must be my new gardener for the orangerie!" "I shall show you where you can find everything you need." "You see the watering can over there? 
Grab it and fillit up at the sink! ")))
  (UserInterface|Viewport|AddtoViewport _returnvalue_3 0)
  (bind _returnvalue_4 (Actor|GetActorOfClass "/Game/Blueprints/BP_Eugen.BP_Eugen_C"))
  (Variables|Default|SetEugenNPC _returnvalue_4))

(event EventTick
  (params (DeltaSeconds :type Float%20%28single-precision%29)))

(fn ConstructionScript)

(fn TutorialCounter
  (bind _result (Math|Integer|IncrementInt (Variables|Default|GetTutorialWateringCounter))
    (:%20%20
      (if (>= _result 3)
        (bind _returnvalue (UserInterface|CreateWidget "/Game/UI/W_TutorialBox.W_TutorialBox_C" 0 (Utilities|Array|MakeArray "Very good! 
Water them when you have to." "Oh and don't forget to harvest the fruits. 
I need them for my guests you know?" "Those trees are from africa. 
You can imagine how important it is to keep the fruits!" "I'll come back later. 
See you!")))
        (UserInterface|Viewport|AddtoViewport _returnvalue 0)
        (bind _outactors (Actor|GetAllActorsOfClass "/Game/Blueprints/Werkzeug/BP_BaseTree.BP_BaseTree_C"))
        (for _array_element _outactors
          (Default|EndTutorial _array_element)
          (CallFunction|EugenMoveAway))))))

(fn StopTreeTimers
  (for _array_element (Variables|Default|GetTrees)
    (Utilities|IsValid _array_element
      (:Is%20Valid
        (Utilities|Time|PauseTimerbyHandle (Variables|/Game/Blueprints/Werkzeug/BP_BaseTree.BP_BaseTree_C|GetDryingTimerHandle _array_element))
        (Utilities|Time|PauseTimerbyHandle (Variables|/Game/Blueprints/Werkzeug/BP_BaseTree.BP_BaseTree_C|GetReifeTimer _array_element))))))

(fn StartTreeTimers
  (for _array_element (Variables|Default|GetTrees)
    (Utilities|IsValid _array_element
      (:Is%20Valid
        (Utilities|Time|UnpauseTimerbyHandle (Variables|/Game/Blueprints/Werkzeug/BP_BaseTree.BP_BaseTree_C|GetDryingTimerHandle _array_element))
        (Utilities|Time|UnpauseTimerbyHandle (Variables|/Game/Blueprints/Werkzeug/BP_BaseTree.BP_BaseTree_C|GetReifeTimer _array_element))))))