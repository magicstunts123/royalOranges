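; Prinz Eugen NPC who leaves and returns with paintings, inspecting the player's trees on each visit, with a flipbook sprite switched by movement.
; DialogueGate is a step-by-step state machine chaining camera blends, AI moves to three trees and dialogue boxes flagged to trigger his next action.
; A dead tree costs him the painting; otherwise he hangs it and saves an achievement.
; Each visit ends by removing dead trees and checking win or loss.
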(event Custom|GoAway
  (AI|AIMoveTo self "0, 0, 0" (Variables|Default|GetTargetAway) 5.0 false))

(event Custom|ComeBack
  (CallFunction|GetPicture)
  (AI|AIMoveTo self "0, 0, 0" (Variables|Default|GetTargetBack) 5.0 false
    (:OnSuccess
      (Math|Integer|IncrementInt (Variables|Default|GetPaintingCounter)
        (:%20%20
          (switch int (Variables|Default|GetPaintingCounter)
            (:1
              (bind _returnvalue (UserInterface|CreateWidget "/Game/UI/W_TutorialBox.W_TutorialBox_C" 0 (Utilities|Array|MakeArray "Dominique! 
I am back!" "I hope everything is alright?" "Let's take a look!") 0 true))
              (UserInterface|Viewport|AddtoViewport _returnvalue 0))
            (:2
              (bind _returnvalue_2 (UserInterface|CreateWidget "/Game/UI/W_TutorialBox.W_TutorialBox_C" 0 (Utilities|Array|MakeArray "Dominique! 
I am back!" "I hope everything is alright?" "Let's take a look!") 0 true))
              (UserInterface|Viewport|AddtoViewport _returnvalue_2 0))
            (:3
              (bind _returnvalue_3 (UserInterface|CreateWidget "/Game/UI/W_TutorialBox.W_TutorialBox_C" 0 (Utilities|Array|MakeArray "Dominique! 
I am back!" "I hope everything is alright?" "Let's take a look!") 0 true))
              (UserInterface|Viewport|AddtoViewport _returnvalue_3 0))))))))

(event Custom|ControlTrees
  (params (TreeIndex :type Integer))
  (bind _trees (Variables|Default|GetTrees))
  (bind _output (Utilities|Array|Get(acopy) _trees TreeIndex))
  ;[1 1 1] checking trees
  (Utilities|IsValid _output
    (:Is%20Valid
      (AI|AIMoveTo self "0, 0, 0" (Utilities|Array|Get(acopy) (Variables|Default|GetTreesPoints) TreeIndex) 5.0 false
        (:OnSuccess
          (Utilities|FlowControl|Delay 2.0)
          (switch Utilities|FlowControl|Switch|SwitchonE_TreeState (Variables|/Game/Blueprints/Werkzeug/BP_BaseTree.BP_BaseTree_C|GetState _output)
            (:NewEnumerator0
              (bind _returnvalue (UserInterface|CreateWidget "/Game/UI/W_TutorialBox.W_TutorialBox_C" 0 (Utilities|Array|MakeArray "Mhmm..." "This one looks good!") 0 true))
              (UserInterface|Viewport|AddtoViewport _returnvalue 0))
            (:NewEnumerator1
              (bind _returnvalue_2 (UserInterface|CreateWidget "/Game/UI/W_TutorialBox.W_TutorialBox_C" 0 (Utilities|Array|MakeArray "Mhmm..." "This one has fruits! 
You should collect them as soon as possible!") 0 true))
              (UserInterface|Viewport|AddtoViewport _returnvalue_2 0))
            (:NewEnumerator2
              (bind _returnvalue_3 (UserInterface|CreateWidget "/Game/UI/W_TutorialBox.W_TutorialBox_C" 0 (Utilities|Array|MakeArray "Mhmm..." "I thought you know what you are doing. " "Please remove that rotten fruits before it gets worse!") 0 true))
              (UserInterface|Viewport|AddtoViewport _returnvalue_3 0))
            (:NewEnumerator3
              (CallFunction|LoosePicture)
              (bind _returnvalue_4 (UserInterface|CreateWidget "/Game/UI/W_TutorialBox.W_TutorialBox_C" 0 (Utilities|Array|MakeArray "Mhmm..." "Oh. My. God." "My disappointment is immeasurable and my day is ruined!" "I'll take this one outside personally!") 0 true false))
              (UserInterface|Viewport|AddtoViewport _returnvalue_4 0))))))
    (:Is%20Not%20Valid
      (CallFunction|DialogueGate))))

(event Custom|DialogueGate
  (bind _returnvalue (Game|GetGameInstance))
  (bind _returnvalue_2 (Game|GetGameInstance))
  (bind _returnvalue_3 (Game|GetGameInstance))
  (bind _paintingcounter (Variables|Default|GetPaintingCounter))
  (bind _asbelvedere_instance (Utilities|Casting|CastToBelvedereInstance _returnvalue_3))
  (bind _asbelvedere_instance_2 (Utilities|Casting|CastToBelvedereInstance _returnvalue))
  (bind _asbelvedere_instance_3 (Utilities|Casting|CastToBelvedereInstance _returnvalue_2))
  (switch int (Variables|Default|GetDialoguePart)
    (:0
      (Variables|Default|SetDialoguePart 1)
      (Game|Player|SetViewTargetwithBlend (Game|GetPlayerController 0) self 2.0 "VTBlend_Linear" 0.0 false)
      (Utilities|FlowControl|Delay 2.0)
      (CallFunction|ControlTrees))
    (:1
      (Variables|Default|SetDialoguePart 2)
      (CallFunction|ControlTrees 1))
    (:2
      (Variables|Default|SetDialoguePart 3)
      (CallFunction|ControlTrees 2))
    (:3
      (Variables|Default|SetDialoguePart 4)
      (if (Variables|Default|GetShouldHavePaintingToCollecting)
        (AI|AIMoveTo self (Transformation|GetActorLocation (Utilities|Array|Get(acopy) (Variables|Default|GetPaintingsLocations) (- (Variables|Default|GetPaintingCounter) 1))) 0 1e+01 true
          (:OnSuccess
            _)
          (:OnFail
            _))
        (Rendering|SetVisibility (Variables|/Game/Assets/Prototype/BP_Bilderrahmen.BP_Bilderrahmen_C|GetScene (Utilities|Array|Get(acopy) (Variables|Default|GetPaintingsLocations) (- _paintingcounter 1))) true true)
        (Rendering|SetVisibility (Variables|Default|GetBild) false false)
        (switch int (Variables|Default|GetPaintingCounter)
          (:1
            (bind _returnvalue_4 (UserInterface|CreateWidget "/Game/UI/W_TutorialBox.W_TutorialBox_C" 0 (Utilities|Array|MakeArray "Ah this Picture looks good there!" "I will never write down a testament you know?") 0 true))
            (UserInterface|Viewport|AddtoViewport _returnvalue_4 0)
            (Default|UnlockAchievement (Variables|/Game/Blueprints/BelvedereInstance.BelvedereInstance_C|GetAs%20BP%20Belvedere%20Savegame _asbelvedere_instance_2) "NewEnumerator2")
            (Default|SaveGame _asbelvedere_instance_2))
          (:2
            (bind _returnvalue_5 (UserInterface|CreateWidget "/Game/UI/W_TutorialBox.W_TutorialBox_C" 0 (Utilities|Array|MakeArray "Ah this Picture looks good there!" "I wonder what Johann Bernhard Fischer is doing these days. 
Maybe i should invite him and give him one of these paintings." "That's how people remember me.") 0 true))
            (UserInterface|Viewport|AddtoViewport _returnvalue_5 0)
            (Default|UnlockAchievement (Variables|/Game/Blueprints/BelvedereInstance.BelvedereInstance_C|GetAs%20BP%20Belvedere%20Savegame _asbelvedere_instance_3) "NewEnumerator1")
            (Default|SaveGame _asbelvedere_instance_3))
          (:3
            (bind _returnvalue_6 (UserInterface|CreateWidget "/Game/UI/W_TutorialBox.W_TutorialBox_C" 0 (Utilities|Array|MakeArray "Ah this Picture looks good there!" "It took 10 years to build my \"olymp\" here." "Hildebrandt did a good job!") 0 true))
            (UserInterface|Viewport|AddtoViewport _returnvalue_6 0)
            (Default|UnlockAchievement (Variables|/Game/Blueprints/BelvedereInstance.BelvedereInstance_C|GetAs%20BP%20Belvedere%20Savegame _asbelvedere_instance) "NewEnumerator0")
            (Default|SaveGame _asbelvedere_instance)))
        (Default|UpdatePaintingCounter (Variables|/Game/Blueprints/BP_EugenMode.BP_EugenMode_C|GetHUD (.AsBP%20Eugen%20Mode (Utilities|Casting|CastToBP_EugenMode (Game|GetGameMode)))) (Utilities|Text|ToText(Integer) (Variables|Default|GetPaintingCounter)))
        (else
          (bind _returnvalue_7 (UserInterface|CreateWidget "/Game/UI/W_TutorialBox.W_TutorialBox_C" 0 (Utilities|Array|MakeArray "Now i have to get a new painting! 
") 0 true))
          (UserInterface|Viewport|AddtoViewport _returnvalue_7 0)
          (Math|Integer|DecrementInt _paintingcounter))))
    (:4
      ;[1 1 1] Gesprächsende
      (Game|Player|SetViewTargetwithBlend (Game|GetPlayerController 0) (Game|Player|GetPlayerPawn 0) 2.0 "VTBlend_Linear" 0.0 false)
      (bind _returnvalue_8 (UserInterface|CreateWidget "/Game/UI/W_TutorialBox.W_TutorialBox_C" 0 (Utilities|Array|MakeArray "Okay. 
I got to go now!")))
      (UserInterface|Viewport|AddtoViewport _returnvalue_8 0)
      (Variables|Default|SetDialoguePart 0)
      (for _array_element (Variables|Default|GetTrees)
        (Utilities|IsValid _array_element
          (:Is%20Valid
            (switch Utilities|FlowControl|Switch|SwitchonE_TreeState (Variables|/Game/Blueprints/Werkzeug/BP_BaseTree.BP_BaseTree_C|GetState _array_element)
              (:NewEnumerator3
                (Actor|DestroyActor _array_element))))))
      (if (CallFunction|CheckifGameOver)
        (bind _returnvalue_9 (UserInterface|CreateWidget "/Game/UI/W_Lost.W_Lost_C"))
        (UserInterface|Viewport|AddtoViewport _returnvalue_9 0)
        (else
          (Default|EugenMoveAway (.AsBP%20Eugen%20Mode (Utilities|Casting|CastToBP_EugenMode (Game|GetGameMode))))
          (if (>= (Variables|Default|GetPaintingCounter) 3)
            (Development|PrintString "GameOver")
            (Utilities|FlowControl|Delay 3.0)
            (bind _returnvalue_10 (UserInterface|CreateWidget "/Game/UI/W_Won.W_Won_C"))
            (UserInterface|Viewport|AddtoViewport _returnvalue_10 0)))))))

(event EventTick
  (params (DeltaSeconds :type Float%20%28single-precision%29))
  (bind _sprite (Variables|Default|GetSprite))
  (if (== (Math|Vector|VectorLength (Transformation|GetVelocity)) 0.0)
    (Sprite|SetFlipbook _sprite "/Game/Assets/Prinz_Eugen_Thinking_Flipbook.Prinz_Eugen_Thinking_Flipbook")
    (else
      (Sprite|SetFlipbook _sprite "/Game/Assets/Prinz_Eugen1.Prinz_Eugen1"))))

(event Collision|EventActorBeginOverlap
  (params (OtherActor :type Actor%20Object%20Reference)))

(fn ConstructionScript)

(fn GetPicture
  (Variables|Default|SetShouldHavePaintingToCollecting true)
  (Rendering|SetVisibility (Variables|Default|GetBild) true false))

(fn LoosePicture
  (bind _bild (Variables|Default|GetBild))
  (Variables|Default|SetShouldHavePaintingToCollecting false)
  (Physics|SetSimulatePhysics _bild true)
  (Rendering|SetVisibility _bild false false)
  (Game|SpawnActorfromClass "/Game/Blueprints/GC_BP_Bilderrahmen_Blueprint.GC_BP_Bilderrahmen_Blueprint_C" (Transformation|GetWorldTransform _bild) "AdjustIfPossibleButAlwaysSpawn" "MultiplyWithRoot" 0 0))

(fn CheckifGameOver
  (bind _array_element (Utilities|Array|ForEachLoopwithBreak (Variables|Default|GetTrees) :!label _label)
    (:LoopBody
      (Utilities|IsValid _array_element
        (:Is%20Valid
          (LocalVariables|SetL_ShouldLoose? false)
          (goto _label Break))
        (:Is%20Not%20Valid
          (LocalVariables|SetL_ShouldLoose? true))))
    (:Completed
      (return (LocalVariables|GetL_ShouldLoose?)))))