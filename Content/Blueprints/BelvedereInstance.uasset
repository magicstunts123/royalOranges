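; BelvedereInstance manages the game's single save slot and records achievement unlocks.
; On Init it loads and caches the BP_BelvedereSavegame, or creates and writes a fresh one without caching it.
; ResetSave deletes the slot and reuses that creation path, leaving the cached reference untouched.
; UnlockAchievement maps each named achievement, such as artworks, to an Unlockables entry, sets it true and immediately saves the cached object.
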(event Custom|SaveGame
  (SaveGame|SaveGametoSlot (Variables|Default|GetAs%20BP%20Belvedere%20Savegame) "save"))

(event Custom|UnlockAchievement
  (params (Achievement :type E_Achievement%20Enum :default "NewEnumerator0"))
  (bind _as_bp_belvedere_savegame (Variables|Default|GetAs%20BP%20Belvedere%20Savegame))
  (bind _unlockables (Variables|/Game/Blueprints/BP_BelvedereSavegame.BP_BelvedereSavegame_C|GetUnlockables _as_bp_belvedere_savegame))
  (switch Utilities|FlowControl|Switch|SwitchonE_Achievement Achievement
    (:NewEnumerator0
      (Utilities|Struct|SetmembersinS_Savestruct (Utilities|Array|Get(acopy) _unlockables) true))
    (:NewEnumerator1
      (Utilities|Struct|SetmembersinS_Savestruct (Utilities|Array|Get(acopy) _unlockables 1) true))
    (:NewEnumerator2
      (Utilities|Struct|SetmembersinS_Savestruct (Utilities|Array|Get(acopy) _unlockables 2) true))
    (:NewEnumerator3
      (Utilities|Struct|SetmembersinS_Savestruct (Utilities|Array|Get(acopy) _unlockables 3) true))
    (:NewEnumerator4
      (Utilities|Struct|SetmembersinS_Savestruct (Utilities|Array|Get(acopy) _unlockables 4) true)))
  (CallFunction|SaveGame))

(event Custom|ResetSave
  (SaveGame|DeleteGameinSlot "save")
  (bind _returnvalue (SaveGame|CreateSaveGameObject "/Game/Blueprints/BP_BelvedereSavegame.BP_BelvedereSavegame_C"))
  (SaveGame|SaveGametoSlot _returnvalue "save"))

(event EventInit
  (bind _returnvalue (SaveGame|DoesSaveGameExist "save"))
  (if _returnvalue
    (bind _returnvalue_2 (SaveGame|LoadGamefromSlot "save"))
    (bind _asbp_belvedere_savegame (Utilities|Casting|CastToBP_BelvedereSavegame _returnvalue_2))
    (Variables|Default|SetAs%20BP%20Belvedere%20Savegame _asbp_belvedere_savegame)
    (else
      (bind _returnvalue_3 (SaveGame|CreateSaveGameObject "/Game/Blueprints/BP_BelvedereSavegame.BP_BelvedereSavegame_C"))
      (SaveGame|SaveGametoSlot _returnvalue_3 "save"))))